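; BP_Pushable is a component that lets its owner actor be pushed by a displacement when the given force meets its required threshold.
; Push line-traces ahead and recursively pushes any pushable blocker with the remaining force, so chains move only if force suffices.
; On success it offsets the owner without sweep and triggers an optional footstep sound; failures can return the blocking actor.
; Enable and disable functions toggle pushing.
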(fn `Disable Push`
  (set `self.Push Enabled` false))

(fn `Enable Push`
  (set `self.Push Enabled` true))

(fn `Push`
  (params (Despl :type "Vector Structure") (Fuerza :type Integer))
  (returns (Success :type Boolean) (Obstaculo :type "Actor Object Reference"))
  (bind _returnvalue (`Actor.GetComponentByClass` (`self.GetOwner`) "/Game/Components/FootSetepSound.FootSetepSound_C"))
  (bind _returnvalue_2 (+ (`Actor.K2_GetActorLocation` (`self.GetOwner`)) (0.0 0.0 50.0)))
  (if (`self.Push Enabled`)
    (if (>= (`local.Fuerza`) (`self.Fuerza Necesaria`))
      (bind (_outhit _returnvalue_3) (`KismetSystemLibrary.LineTraceSingle` _returnvalue_2 (+ _returnvalue_2 (`local.Despl`)) "TraceTypeQuery1"))
      (if _returnvalue_3
        (bind _returnvalue_4 (`Actor.GetComponentByClass` (`.HitActor` (`GameplayStatics.BreakHitResult` _outhit)) "BP_Pushable_C"))
        (`/Engine/EditorBlueprintResources/StandardMacros.IsValid` _returnvalue_4
          (:`Is Valid`
            (bind (_success _obstaculo) (`self.Push` _returnvalue_4 (`local.Despl`) (- (`local.Fuerza`) (`self.Fuerza Necesaria`))))
            (if _success
              _
              (else
                (return false _obstaculo))))
          (:`Is Not Valid`
            (return false (`.HitActor` (`GameplayStatics.BreakHitResult` _outhit))))))
      (`Actor.K2_AddActorWorldOffset` (`self.GetOwner`) (`local.Despl`) false false)
      (`/Engine/EditorBlueprintResources/StandardMacros.IsValid` _returnvalue
        (:`Is Valid`
          (bind _asfoot_setep_sound (cast `/Game/Components/FootSetepSound` _returnvalue))
          (`/Game/Components/FootSetepSound.On Foot` _asfoot_setep_sound))
        (:`Is Not Valid`
          _))
      (return true null)
      (else
        (return false null)))
    (else
      (return false null))))