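; BP_Columna is a column actor that temporarily swaps its material when notified that it is in the way.
; The OnEstasEnMedio event applies MaterialEstorbando, then a 0.5-second retriggerable delay restores the default Material, so repeated calls keep the obstructing look active.
; ChangeMaterial sets element 0 on every static mesh component if the material is valid, and the construction script uses it to apply the default.
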(event `/Game/Blueprints/Interfaces/BPI_AmableConCamara.OnEstasEnMedio`
  (`self.Change Material` (`self.Material Estorbando`))
  (`KismetSystemLibrary.RetriggerableDelay` 0.5)
  (`self.Change Material` (`self.Material`)))

(fn `Change Material`
  (params (Material :type "Material Object Reference"))
  (`/Engine/EditorBlueprintResources/StandardMacros.IsValid` Material
    (:`Is Valid`
      (for _array_element (`self.K2_GetComponentsByClass` "/Script/Engine.StaticMeshComponent")
        (`PrimitiveComponent.SetMaterial` _array_element 0 Material)))))

(fn `UserConstructionScript`
  (`self.Change Material` (`self.Material`)))