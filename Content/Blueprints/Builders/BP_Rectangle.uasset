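; BP_Rectangle is a builder actor that lays out the hollow outline of a rectangle from BlockEntity actors, sized by XSize and YSize.
; The construction script runs one loop for the rows along X and another for the side columns, which overlap at the Y=0 corners.
; CreateObject checks the class, then adds a child actor component at each tile position on a 100-unit grid.
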(fn `Create Object`
  (params (`Tile X` :type Integer) (`Tile Y` :type Integer))
  (if (`KismetSystemLibrary.IsValidClass` (`self.Block Entity`))
    (bind _returnvalue (`AddComponent|NODE_AddChildActorComponent-0` :`RelativeTransform` (`KismetMathLibrary.Conv_VectorToTransform` (`KismetMathLibrary.MakeVector` (* (`local.Tile X`) 100.0) (* (`local.Tile Y`) 100.0)))))
    (`ChildActorComponent.SetChildActorClass` _returnvalue (`self.Block Entity`))))

(fn `UserConstructionScript`
  (`|ExecutionSequence`
    (:`then_0`
      (for _index (range (`self.X size`))
        (`self.Create Object` _index)
        (`self.Create Object` _index (- (`self.Y size`) 1))))
    (:`then_1`
      (for _index_2 (range (+ (- (`self.Y size`) 2) 1))
        (`self.Create Object` 0 _index_2)
        (`self.Create Object` (- (`self.X size`) 1) _index_2)))))