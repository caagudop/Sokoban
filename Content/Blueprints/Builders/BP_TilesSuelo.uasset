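; BP_TilesSuelo is a builder actor that lays out a grid of floor tiles from a text map.
; Its Construction Script reads each Description string as a row along X and each character as a tile along Y.
; CodeToClass maps characters to wood, ceramic or metal floor classes, and CreateObject adds valid ones as Child Actor Components at 100-unit spacing.
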(fn `Code To Class`
  (params (Code :type String))
  (returns (`Object Class` :type "Actor Class Reference"))
  (switch `string` Code
    (:`Default`
      (return null))
    (:`M`
      (return "/Game/Blueprints/Suelos/Suelo_Madera.Suelo_Madera_C"))
    (:`C`
      (return "/Game/Blueprints/Suelos/Suelo_Ceramica.Suelo_Ceramica_C"))
    (:`L`
      (return "/Game/Blueprints/Suelos/Suelo_Metal.Suelo_Metal_C"))))

(fn `Create Object`
  (params (`Tile X` :type Integer) (`Tile Y` :type Integer) (`Entity Class` :type "Actor Class Reference"))
  (locals (NumCadena :type Integer) (NumChar :type Integer))
  (if (`KismetSystemLibrary.IsValidClass` `Entity Class`)
    (bind _returnvalue (`AddComponent|NODE_AddChildActorComponent-0` :`RelativeTransform` (`KismetMathLibrary.MakeTransform` (`KismetMathLibrary.MakeVector` (* (`local.Tile X`) 100.0) (* (`local.Tile Y`) 100.0)))))
    (`ChildActorComponent.SetChildActorClass` _returnvalue (`local.Entity Class`))))

(fn `UserConstructionScript`
  (locals (NumCadena :type Integer) (NumChar :type Integer))
  (for (_array_element _array_index) (`self.Description`)
    (set `local.NumCadena` _array_index)
    (for (_array_element_2 _array_index_2) (`KismetStringLibrary.GetCharacterArrayFromString` _array_element)
      (set `local.NumChar` _array_index_2)
      (bind _object_class (`self.Code To Class` _array_element_2))
      (`self.Create Object` (`local.NumCadena`) (`local.NumChar`) _object_class))))