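; BP_Landing is a Sokoban target tile that detects when a box (BP_Caja) enters or leaves its BoxCollider.
; On begin and end overlap it calls OnBoxLanded or OnBoxUnlanded on the BP_SokobanLogic game mode.
; When the Bloqueante flag is set, a box that lands on it is also made non-pushable.
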(event `self.Box collider.OnComponentBeginOverlap`
  (params (OverlappedComponent :type "PrimitiveComponent Object Reference") (OtherActor :type "Actor Object Reference") (OtherComp :type "PrimitiveComponent Object Reference") (OtherBodyIndex :type Integer) (bFromSweep :type Boolean) (SweepResult :type "HitResult Structure (by ref)"))
  (bind _asbp_caja (cast `/Game/Blueprints/BP_Caja` OtherActor))
  (bind _asbp_sokoban_logic (cast `/Game/Blueprints/BP_SokobanLogic` (`GameplayStatics.GetGameMode`)))
  (`/Game/Blueprints/BP_SokobanLogic.OnBoxLanded` _asbp_sokoban_logic)
  (if (`self.Bloqueante`)
    (`/Game/Blueprints/BP_Caja.Set Is Pushable` _asbp_caja false)))

(event `self.Box collider.OnComponentEndOverlap`
  (params (OverlappedComponent :type "PrimitiveComponent Object Reference") (OtherActor :type "Actor Object Reference") (OtherComp :type "PrimitiveComponent Object Reference") (OtherBodyIndex :type Integer))
  (cast `/Game/Blueprints/BP_Caja` OtherActor)
  (bind _asbp_sokoban_logic (cast `/Game/Blueprints/BP_SokobanLogic` (`GameplayStatics.GetGameMode`)))
  (`/Game/Blueprints/BP_SokobanLogic.OnBoxUnlanded` _asbp_sokoban_logic))

(fn `UserConstructionScript`
  (`parent.UserConstructionScript`))