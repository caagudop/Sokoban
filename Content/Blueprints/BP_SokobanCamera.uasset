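; Follow camera for a Sokoban-style game that keeps its target in view around obstacles.
; Each tick it smoothly turns toward the target's eye height and moves toward a chosen position.
; It steps from the initial target offset toward an overhead fallback, taking the first point with a clear visibility trace.
; Blockers implementing BPI_AmableConCamara receive an in-the-way message and count as see-through.
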(event `self.ReceiveBeginPlay`
  (`self.Change Target Actor` (`self.Target`)))

(event `self.ReceiveTick`
  (params (DeltaSeconds :type "Float (single-precision)"))
  (`/Engine/EditorBlueprintResources/StandardMacros.IsValid` (`self.Target`)
    (:`Is Valid`
      (`self.UpdateRotation`)
      (`self.UpdatePostion`))))

(fn `Can See Target From`
  (params (Location :type "Vector Structure"))
  (returns (`Is Visible` :type Boolean))
  (bind (_outhit _returnvalue) (`KismetSystemLibrary.LineTraceSingle` Location (`self.Get Look At Position`) "TraceTypeQuery1" false (`|MakeArray` (`self.Target`))))
  (if _returnvalue
    (bind (_bblockinghit _binitialoverlap _time _distance _location _impactpoint _normal _impactnormal _physmat _hitactor) (`GameplayStatics.BreakHitResult` _outhit))
    (if (`KismetSystemLibrary.DoesImplementInterface` _hitactor "/Game/Blueprints/Interfaces/BPI_AmableConCamara.BPI_AmableConCamara_C")
      (message `/Game/Blueprints/Interfaces/BPI_AmableConCamara.OnEstasEnMedio` _hitactor)
      (return true)
      (else
        (return false)))
    (else
      (return true))))

(fn `Change Target Actor`
  (params (`New Target Actor` :type "Actor Object Reference"))
  (bind _returnvalue (- (`self.K2_GetActorLocation`) (`self.Get Look At Position`)))
  (bind _output_get (set `self.Target` `New Target Actor`))
  (`/Engine/EditorBlueprintResources/StandardMacros.IsValid` _output_get
    (:`Is Valid`
      (set `self.TargetOffset` _returnvalue)
      (set `self.Target Distance` (`KismetMathLibrary.VSize` _returnvalue)))))

(fn `Get Look At Position`
  (returns (Position :type "Vector Structure"))
  (return (+ (`self.K2_GetActorLocation` (`self.Target`)) (`KismetMathLibrary.MakeVector` 0.0 0.0 (`self.Target Eyes Height`)))))

(fn `UpdatePostion`
  (locals (`Selected Position` :type "Vector Structure"))
  (set `local.Selected Position` (`self.Get Last Resource Position`))
  (for _index (range 11)
    (bind _returnvalue (`KismetMathLibrary.VLerp` (`self.Get Natural Position`) (`self.Get Last Resource Position`) (`KismetMathLibrary.NormalizeToRange` (`KismetMathLibrary.Conv_IntToDouble` _index) 0.0 10.0)))
    (bind _is_visible (`self.Can See Target From` _returnvalue))
    (if _is_visible
      (set `local.Selected Position` _returnvalue)
      (break)))
  (`self.K2_SetActorLocation` (`KismetMathLibrary.VLerp` (`self.K2_GetActorLocation`) (`local.Selected Position`) (* (`self.Translation Speed`) (`GameplayStatics.GetWorldDeltaSeconds`)))))

(fn `UpdateRotation`
  (`SceneComponent.K2_SetWorldRotation` (`self.SceneComponent`) (`KismetMathLibrary.RLerp` (`self.K2_GetActorRotation`) (`KismetMathLibrary.FindLookAtRotation` (`self.K2_GetActorLocation`) (`self.Get Look At Position`)) (* (`self.Rotation Speed`) (`GameplayStatics.GetWorldDeltaSeconds`))) false false))

(fn `UserConstructionScript`)