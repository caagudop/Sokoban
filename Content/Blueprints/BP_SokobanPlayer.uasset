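; Player actor for a Sokoban puzzle: WASD attempts one 100-unit grid step and snaps rotation to that direction, and R reloads the level.
; TryMoveTowards delegates movement to the player's own Pushable component, pushing with a fixed force.
; Success fires PlayerMoved, while failure sends a bump message to any valid obstacle.
; BeginPlay creates the main HUD; an older line-trace movement path using TryPush remains unreachable.
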(event `self.ReceiveBeginPlay`
  (bind _returnvalue (`|CreateWidget` "/Game/HUD/MainHUD.MainHUD_C"))
  (`UserWidget.AddToViewport` _returnvalue 0))

(event `Key|A`
  (params (Key :type "Key Structure"))
  ;[1 1 1] Input Jugador
  (:`Pressed`
    (`self.Try Move Towards` (0.0 -100.0 0.0))
    (`self.K2_SetActorRotation` (struct :`Yaw` -90.0))))

(event `Key|D`
  (params (Key :type "Key Structure"))
  ;[1 1 1] Input Jugador
  (:`Pressed`
    (`self.Try Move Towards` (0.0 100.0 0.0))
    (`self.K2_SetActorRotation` (struct :`Yaw` 90.0))))

(event `Key|W`
  (params (Key :type "Key Structure"))
  ;[1 1 1] Input Jugador
  (:`Pressed`
    (`self.Try Move Towards` (100.0 0.0 0.0))
    (`self.K2_SetActorRotation` (struct))))

(event `Key|S`
  (params (Key :type "Key Structure"))
  ;[1 1 1] Input Jugador
  (:`Pressed`
    (`self.Try Move Towards` (-100.0 0.0 0.0))
    (`self.K2_SetActorRotation` (struct :`Yaw` 180.0))))

(event `Key|R`
  (params (Key :type "Key Structure"))
  ;[1 1 1] Restart level
  (:`Pressed`
    (bind _returnvalue (`GameplayStatics.GetCurrentLevelName` true))
    (`GameplayStatics.OpenLevel` (`KismetStringLibrary.Conv_StringToName` _returnvalue))))

(fn `Try Bump`
  (params (Object :type "Actor Object Reference"))
  (message `/Game/Blueprints/Interfaces/BPI_Chocable.SomethingBump` Object))

(fn `Try Move Towards`
  (params (Desp :type "Vector Structure"))
  (returns (Sucess :type Boolean))
  (bind (_success _obstaculo) (`/Game/Components/BP_Pushable.Push` (`self.Pushable`) Desp 2))
  (if _success
    (`self.PlayerMoved`)
    (return true)
    (else
      (`/Engine/EditorBlueprintResources/StandardMacros.IsValid` _obstaculo
        (:`Is Valid`
          (`self.Try Bump` _obstaculo))
        (:`Is Not Valid`
          _))
      (return false))))

(fn `Try Push`
  (params (Object :type "Actor Object Reference") (Desp :type "Vector Structure"))
  (returns (Pushed :type Boolean))
  (bind _returnvalue (`self.GetComponentByClass` Object "/Game/Components/BP_Pushable.BP_Pushable_C"))
  (`/Engine/EditorBlueprintResources/StandardMacros.IsValid` _returnvalue
    (:`Is Valid`
      (bind _success (`/Game/Components/BP_Pushable.Push` _returnvalue (`local.Desp`) 2))
      (return _success))
    (:`Is Not Valid`
      (return false))))

(fn `UserConstructionScript`)