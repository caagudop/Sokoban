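; BP_SokobanLogic tracks move count and box placement for a Sokoban puzzle level.
; On BeginPlay it counts all BP_Caja boxes and binds to the player's move event, which increments a local counter and the total in the BP_Sokoban_Data game instance.
; OnBoxLanded and OnBoxUnlanded maintain the placed-box count; when it matches the box total on a landing, every box becomes non-pushable.
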(event `self.ReceiveBeginPlay`
  (`|ExecutionSequence`
    (:`then_0`
      (bind _asbp_sokoban_player (cast `/Game/Blueprints/BP_SokobanPlayer` (`GameplayStatics.GetPlayerPawn` 0)))
      (add `/Game/Blueprints/BP_SokobanPlayer.PlayerMoved` _asbp_sokoban_player (delegate `Player Moved`)))
    (:`then_1`
      (bind _outactors (`GameplayStatics.GetAllActorsOfClass` "/Game/Blueprints/BP_Caja.BP_Caja_C"))
      (set `self.numCajas` (`KismetArrayLibrary.Array_Length` _outactors)))))

(event `Player Moved`
  (`/Engine/EditorBlueprintResources/StandardMacros.IncrementInt` (`self.Num Movements`)
    (:`  `
      (bind _asbp_sokoban_data (cast `/Game/Blueprints/BP_Sokoban_Data` (`GameplayStatics.GetGameInstance`)))
      (`/Engine/EditorBlueprintResources/StandardMacros.IncrementInt` (`/Game/Blueprints/BP_Sokoban_Data.Total Movements` _asbp_sokoban_data)))))

(fn `OnBoxLanded`
  (`/Engine/EditorBlueprintResources/StandardMacros.IncrementInt` (`self.NumCajasColocadas`)
    (:`  `
      (if (== (`self.numCajas`) (`self.NumCajasColocadas`))
        (bind _outactors (`GameplayStatics.GetAllActorsOfClass` "/Game/Blueprints/BP_Caja.BP_Caja_C"))
        (for _array_element _outactors
          (`/Game/Blueprints/BP_Caja.Set Is Pushable` _array_element false))))))

(fn `OnBoxUnlanded`
  (`/Engine/EditorBlueprintResources/StandardMacros.DecrementInt` (`self.NumCajasColocadas`)))

(fn `UserConstructionScript`)