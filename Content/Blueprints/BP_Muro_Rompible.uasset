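; Breakable wall actor that shows progressive damage and destroys itself after enough bumps.
; Each SomethingBump event increments NivelDeRotura and applies the matching entry from the Materiales array to the Cube, or destroys the actor once the level runs past the array.
; The construction script applies the material for the current level, so the number of materials sets how many bumps the wall withstands.
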(event `/Game/Blueprints/Interfaces/BPI_Chocable.SomethingBump`
  (bind _result (`/Engine/EditorBlueprintResources/StandardMacros.IncrementInt` (`self.Nivel de rotura`))
    (:`  `
      (if (< _result (`KismetArrayLibrary.Array_Length` (`self.Materiales`)))
        (`self.Update Material`)
        (else
          (`self.K2_DestroyActor`))))))

(fn `Update Material`
  (`PrimitiveComponent.SetMaterial` (`self.Cube`) 0 (`|GetArrayItem` (`self.Materiales`) (`self.Nivel de rotura`))))

(fn `UserConstructionScript`
  (`self.Update Material`))